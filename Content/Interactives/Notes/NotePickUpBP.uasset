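; Interactive note Blueprint that shows and hides an on-screen note widget for reading.
; ReadNote toggles on the IsReading flag, either creating a NotePickUp_Widget in the viewport or removing it from its parent.
; Picking up the note also hides the mouse cursor.
; InteractWith is a stub returning an empty string and does not trigger the toggle.
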(event Custom|TogglePickUpNote
  (if (Variables|Default|GetIsReading?)
    (CallFunction|PutDownNote)
    (else
      (CallFunction|PickUpNote))))

(event Custom|PutDownNote
  (Widget|RemovefromParent (stale Custom|PickUpNote _returnvalue))
  (Variables|Default|SetIsReading? false))

(event Custom|PickUpNote
  (bind _returnvalue (UserInterface|CreateWidget "/Game/Interactives/Notes/NotePickUp_Widget.NotePickUp_Widget_C"))
  (UserInterface|Viewport|AddtoViewport _returnvalue 0)
  (Variables|Default|SetIsReading? true)
  (Variables|/Script/Engine.PlayerController|SetbShowMouseCursor (Game|GetPlayerController 0) false))

(event EventReadNote
  (CallFunction|TogglePickUpNote))

(fn ConstructionScript)

(fn Interactwith
  (params (Player%20Character :type First%20Person%20Character%20Object%20Reference))
  (return ""))